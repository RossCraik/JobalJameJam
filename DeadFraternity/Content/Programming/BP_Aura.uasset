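; BP_Aura is an animated visual actor that makes its static mesh pulse and drift in rotation.
; Each Tick sets a uniform scale from the absolute value of a slow time-based sine, so the mesh swells and shrinks above a minimum size.
; It also adds a small delta-scaled random local rotation, roll included, giving an irregular wobble rather than a steady spin.
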(event EventBeginPlay)

(event Collision|EventActorBeginOverlap
  (params (OtherActor :type Actor%20Object%20Reference)))

(event EventTick
  (params (DeltaSeconds :type Float%20%28single-precision%29))
  (bind _staticmesh (Variables|Default|GetStaticMesh))
  (Transformation|SetRelativeScale3D _staticmesh (* (Class|KismetMathLibrary|VectorOne) (+ (Math|Float|Absolute(Float) (* (Math|Trig|Sin(Radians) (* (Utilities|Time|GetTimeSeconds) 0.25)) 0.4)) 0.8)))
  (Transformation|AddLocalRotation _staticmesh (* (Math|Random|RandomRotator true) (* DeltaSeconds 0.1)) false false))

(fn ConstructionScript)