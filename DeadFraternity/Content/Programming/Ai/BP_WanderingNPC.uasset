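; BP_WanderingNPC is a wandering ghost NPC with a randomized body and face; no movement logic lives in this graph.
; On BeginPlay it picks one of two body meshes, weighted toward the first, then gives its child BP_GhostFace random eyes, mouth and talk speed and starts it talking.
; Tick bobs the body mesh vertically with a time-based sine, scaled by clamped horizontal movement speed plus an idle offset.
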(event Custom|PickBody
  (bind _npc_1 (Variables|Default|GetNPC_1))
  (switch int (Math|Random|RandomIntegerinRange 0 2)
    (:Default
      (Components|StaticMesh|SetStaticMesh _npc_1 "/Game/Characters/NPC_1.NPC_1" :!label _label))
    (:0
      (goto _label))
    (:1
      (Components|StaticMesh|SetStaticMesh _npc_1 "/Game/Characters/NPC_2.NPC_2"))))

(event EventBeginPlay
  (CallFunction|PickBody)
  (bind _asbp_ghost_face (Utilities|Casting|CastToBP_GhostFace (Variables|/Script/Engine.ChildActorComponent|GetChildActor (Variables|Default|GetBP_GhostFace))))
  (Default|SetupFace _asbp_ghost_face (.OutItem (Utilities|Array|Random (Variables|Default|Geteye_array))) (.OutItem (Utilities|Array|Random (Variables|Default|Getmouth_array))) (Math|Random|RandomFloatinRange 0.0 0.2))
  (Default|ToggleTalking _asbp_ghost_face true))

(event EventTick
  (params (DeltaSeconds :type Float%20%28single-precision%29))
  (Transformation|AddLocalOffset (Variables|Default|GetNPC_1) (Math|Vector|MakeVector 0.0 0.0 (* (Math|Trig|Sin(Radians) (Utilities|Time|GetTimeSeconds)) (+ (Math|Float|Clamp(Float) (/ (Class|KismetMathLibrary|VSizeXYSquared (Class|NavMovementComponent|GetVelocityforNavMovement (Variables|Character|GetCharacterMovement))) 666.0) -0.2 0.2) 0.1))) false false))

(event Collision|EventActorBeginOverlap
  (params (OtherActor :type Actor%20Object%20Reference)))

(fn ConstructionScript)