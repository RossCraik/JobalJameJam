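; BP_Collectable is a quest item whose Collect function tells a matching NPC to speak.
; The item's first tag selects the BP_NPC with the same tag, and the first match gets ShouldSpeak set.
; For "The Twins" tag only, it also swaps the player's checklist entry from finding a slice to speaking to The Twins, then destroys itself.
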(fn ConstructionScript)

(fn Collect
  (bind _returnvalue (Game|GetPlayerCharacter 0))
  (bind _tags (Variables|Actor|GetTags))
  (bind _asbp_first_person_character (Utilities|Casting|CastToBP_FirstPersonCharacter _returnvalue))
  (bind _output (Utilities|Array|Get(acopy) _tags))
  (bind _checklist (Variables|/Game/FirstPerson/Blueprints/BP_FirstPersonCharacter.BP_FirstPersonCharacter_C|GetChecklist _asbp_first_person_character))
  (bind _outactors (Actor|GetAllActorsOfClasswithTag "/Game/Programming/BP_NPC.BP_NPC_C" _output))
  (Variables|/Game/Programming/BP_NPC.BP_NPC_C|SetShouldSpeak (Utilities|Array|Get(acopy) _outactors) true)
  (if (== _output "The Twins")
    (Default|RemoveChecklistItem _checklist "Find a Slice")
    (Default|AddChecklistItem _checklist "Speak to The Twins")
    (Actor|DestroyActor)))