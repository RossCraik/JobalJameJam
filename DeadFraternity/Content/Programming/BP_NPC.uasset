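; Ghost NPC that bobs in place and holds typewriter-style conversations with the player.
; On BeginPlay it sets up its child face actor and loads DT_Dialogue rows matching its first tag.
; Talk steps through the current dialogue set, driving WB_Dialogue, speaker-based cameras and facial expressions.
; Ending a set runs hardcoded per-tag quest logic: enabling partner NPCs, updating the checklist and objective count, and swapping the DJ's music.
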(event Custom|Set%20Text
  (bind _talkindex (Variables|Default|GetTalkIndex))
  (bind _eyestates (Variables|Default|GetEyeStates))
  (bind _mouthstates (Variables|Default|GetMouthStates))
  (bind _browstates (Variables|Default|GetBrowStates))
  (bind _output (Utilities|Array|Get(acopy) _browstates _talkindex))
  (bind _output_2 (Utilities|Array|Get(acopy) _eyestates _talkindex))
  (bind _output_3 (Utilities|Array|Get(acopy) _mouthstates _talkindex))
  (bind _output_get (Variables|Default|SetDisplayedText (Utilities|String|Append (Variables|Default|GetDisplayedText) (Utilities|Array|Get(acopy) (Utilities|String|GetCharacterArrayfromString (Utilities|Array|Get(acopy) (Variables|Default|GetDialogue) (Variables|Default|GetTalkIndex))) (Variables|Default|GetCharIndex)))))
  (Rendering|Components|TextRender|SetText (Variables|/Game/Programming/WB_Dialogue.WB_Dialogue_C|GetTalkText (Variables|Default|GetUI)) (Utilities|Text|ToText(String) _output_get))
  (bind _result (Math|Integer|IncrementInt (Variables|Default|GetCharIndex))
    (:%20%20
      (if (== _result (Utilities|Array|Length (Utilities|String|GetCharacterArrayfromString (Utilities|Array|Get(acopy) (Variables|Default|GetDialogue) (Variables|Default|GetTalkIndex)))))
        (Utilities|Time|ClearandInvalidateTimerbyHandle (stale EventTalk _output_get_2))
        (bind _asbp_ghost_face (Utilities|Casting|CastToBP_GhostFace (Variables|/Script/Engine.ChildActorComponent|GetChildActor (Variables|Default|GetBP_GhostFace))))
        (Default|ToggleTalking _asbp_ghost_face false)
        (Utilities|FlowControl|Sequence
          (:then_0
            (if (!= _output_2 -1)
              (Default|EyesChange _asbp_ghost_face _output_2)))
          (:then_1
            (if (!= _output_3 -1)
              (Default|MouthChange _asbp_ghost_face _output_3)))
          (:then_2
            (if (!= _output -1)
              (Default|BrowsChange _asbp_ghost_face _output))))))))

(event EventBeginPlay
  (bind _tags (Variables|Actor|GetTags))
  (bind _output (Utilities|Array|Get(acopy) _tags))
  (Utilities|FlowControl|Sequence
    (:then_0
      ;[0.15 0.15 0.15 0.5] sets ghost face settings
      (bind _asbp_ghost_face (Utilities|Casting|CastToBP_GhostFace (Variables|/Script/Engine.ChildActorComponent|GetChildActor (Variables|Default|GetBP_GhostFace)))
        (:then
          (Default|SetupFace _asbp_ghost_face (Variables|Default|Geteyes_texture) (Variables|Default|Getmouth_texture) (Variables|Default|Gettalk_rate)))
        (:CastFailed
          (Development|PrintString "Failed to find the ghosts face!"))))
    (:then_1
      (bind _outrownames (DataTable|GetDataTableRowNames "/Game/Programming/DT_Dialogue.DT_Dialogue"))
      (for _array_element _outrownames
        (bind _returnvalue (Utilities|GetDataTableRow "/Game/Programming/DT_Dialogue.DT_Dialogue" _array_element)
          (:then
            (if (Utilities|Enum|Equal(Enum) (.talkingto _returnvalue) (Utilities|String|ToString(Name) (Utilities|Array|Get(acopy) (Variables|Actor|GetTags))))
              (Utilities|Array|Add (Variables|Default|GetDialogue) (.currentdialogue _returnvalue))
              (Utilities|Array|Add (Variables|Default|GetSpeakersName) (.speakersname _returnvalue))
              (Utilities|Array|Add (Variables|Default|GetDialogueSets) (.dialoguetiming _returnvalue))
              (Utilities|Array|Add (Variables|Default|GetEyeStates) (.npceyesindex _returnvalue))
              (Utilities|Array|Add (Variables|Default|GetMouthStates) (.npcmouthindex _returnvalue))
              (Utilities|Array|Add (Variables|Default|GetBrowStates) (.npcbrowsindex _returnvalue))
              (Utilities|Array|Add (Variables|Default|GetBubbleColourStates) (.bubblecolour _returnvalue))
              (if (== _output "Punch Bowl")
                (Variables|Default|SetShouldSpeak false)
                (elif (== _output "DJ")
                  (Variables|Default|SetShouldSpeak false))))))))
    (:then_2
      (Variables|Default|Setbob_speed (Math|Random|RandomFloatinRange 0.25 1.0)))))

(event EventTick
  (params (DeltaSeconds :type Float%20%28single-precision%29))
  ;[0.15 0.15 0.15 0.5] idle bobbing
  (Transformation|AddLocalOffset (Variables|Default|GetNPC_1) (Math|Vector|MakeVector 0.0 0.0 (* (Math|Trig|Sin(Radians) (* (Utilities|Time|GetTimeSeconds) (Variables|Default|Getbob_speed))) (/ (Variables|Default|Getbob_speed) 6.0))) false false))

(event EventTalk
  (bind _returnvalue (Game|GetPlayerCharacter 0))
  (bind _returnvalue_2 (Game|GetPlayerCharacter 0))
  (bind _returnvalue_3 (Game|GetPlayerCharacter 0))
  (bind _returnvalue_4 (Game|GetPlayerCharacter 0))
  (bind _returnvalue_5 (Game|GetPlayerCharacter 0))
  (bind _talkindex (Variables|Default|GetTalkIndex))
  (bind _speakersname (Variables|Default|GetSpeakersName))
  (bind _tags (Variables|Actor|GetTags))
  (bind _asbp_first_person_character (Utilities|Casting|CastToBP_FirstPersonCharacter _returnvalue_3))
  (bind _asbp_first_person_character_2 (Utilities|Casting|CastToBP_FirstPersonCharacter _returnvalue_4))
  (bind _asbp_first_person_character_3 (Utilities|Casting|CastToBP_FirstPersonCharacter _returnvalue_5))
  (bind _asbp_first_person_character_4 (Utilities|Casting|CastToBP_FirstPersonCharacter _returnvalue))
  (bind _asbp_first_person_character_5 (Utilities|Casting|CastToBP_FirstPersonCharacter _returnvalue_2))
  (bind _output (Utilities|Array|Get(acopy) _speakersname _talkindex))
  (bind _output_2 (Utilities|Array|Get(acopy) _tags))
  (bind _checklist (Variables|/Game/FirstPerson/Blueprints/BP_FirstPersonCharacter.BP_FirstPersonCharacter_C|GetChecklist _asbp_first_person_character_4))
  (bind _checklist_2 (Variables|/Game/FirstPerson/Blueprints/BP_FirstPersonCharacter.BP_FirstPersonCharacter_C|GetChecklist _asbp_first_person_character_5))
  (bind _checklist_3 (Variables|/Game/FirstPerson/Blueprints/BP_FirstPersonCharacter.BP_FirstPersonCharacter_C|GetChecklist _asbp_first_person_character))
  (bind _checklist_4 (Variables|/Game/FirstPerson/Blueprints/BP_FirstPersonCharacter.BP_FirstPersonCharacter_C|GetChecklist _asbp_first_person_character_2))
  (bind _checklist_5 (Variables|/Game/FirstPerson/Blueprints/BP_FirstPersonCharacter.BP_FirstPersonCharacter_C|GetChecklist _asbp_first_person_character_3))
  (Utilities|Time|ClearandInvalidateTimerbyHandle (Variables|Default|GetTimer))
  (if (Variables|Default|GetShouldSpeak)
    (if (== (Utilities|Array|Get(acopy) (Variables|Default|GetDialogueSets) (+ (Variables|Default|GetTalkIndex) 1)) (Variables|Default|GetCurrentDialogueSet))
      (Math|Integer|IncrementInt (Variables|Default|GetTalkIndex)
        (:%20%20
          (Variables|Default|GetUI
            (:then
              _)
            (:else
              (bind _returnvalue_6 (UserInterface|CreateWidget "/Game/Programming/WB_Dialogue.WB_Dialogue_C" (Game|GetPlayerController 0)))
              (bind _output_get (Variables|Default|SetUI _returnvalue_6))
              (UserInterface|Viewport|AddtoViewport _output_get 0)))
          (Variables|Default|SetDisplayedText "")
          (Variables|Default|SetCharIndex 0)
          (bind _asbp_ghost_face (Utilities|Casting|CastToBP_GhostFace (Variables|/Script/Engine.ChildActorComponent|GetChildActor (Variables|Default|GetBP_GhostFace))))
          (Default|ToggleTalking _asbp_ghost_face true)
          (Class|Border|SetBrushColor (Variables|/Game/Programming/WB_Dialogue.WB_Dialogue_C|GetDialogueBubble (Variables|Default|GetUI)) (Math|Conversions|ToLinearColor(Color) (Utilities|Array|Get(acopy) (Variables|Default|GetBubbleColourStates) (Variables|Default|GetTalkIndex))))
          (bind _returnvalue_7 (Utilities|Time|SetTimerbyEvent (delegate Custom|Set%20Text) (Variables|Default|GetTypeSpeed) true))
          (bind _output_get_2 (Variables|Default|SetTimer _returnvalue_7))
          (Rendering|Components|TextRender|SetText (Variables|/Game/Programming/WB_Dialogue.WB_Dialogue_C|GetNameText (Variables|Default|GetUI)) (Utilities|Text|ToText(String) _output))
          (bind _returnvalue_8 (Actor|GetActorOfClass "/Game/FirstPerson/Blueprints/BP_FirstPersonCharacter.BP_FirstPersonCharacter_C"))
          (if (Utilities|Enum|Equal(Enum) _output "You")
            (Components|Activation|SetActive (Variables|/Game/FirstPerson/Blueprints/BP_FirstPersonCharacter.BP_FirstPersonCharacter_C|GetThirdPersonCamera _returnvalue_8) false false)
            (Components|Activation|SetActive (Variables|/Game/FirstPerson/Blueprints/BP_FirstPersonCharacter.BP_FirstPersonCharacter_C|GetThirdPersonCamera2 _returnvalue_8) true false)
            (goto _label Reset)
            (else
              (Components|Activation|SetActive (Variables|/Game/FirstPerson/Blueprints/BP_FirstPersonCharacter.BP_FirstPersonCharacter_C|GetThirdPersonCamera _returnvalue_8) true false)
              (Components|Activation|SetActive (Variables|/Game/FirstPerson/Blueprints/BP_FirstPersonCharacter.BP_FirstPersonCharacter_C|GetThirdPersonCamera2 _returnvalue_8) false false)
              (goto _label Reset)))))
      (else
        (Utilities|FlowControl|DoOnce false :!label _label
          (:Completed
            (bind _asbp_ghost_face_2 (Utilities|Casting|CastToBP_GhostFace (Variables|/Script/Engine.ChildActorComponent|GetChildActor (Variables|Default|GetBP_GhostFace))))
            (Default|ToggleTalking _asbp_ghost_face_2 false)
            (bind _ui (Variables|Default|GetUI)
              (:then
                (Widget|RemovefromParent _ui))
              (:else
                _))
            (bind _returnvalue_9 (Actor|GetActorOfClass "/Game/FirstPerson/Blueprints/BP_FirstPersonCharacter.BP_FirstPersonCharacter_C"))
            (Default|EndDialogue _returnvalue_9)
            (Variables|Default|SetShouldSpeak false)
            (Math|Integer|IncrementInt (Variables|Default|GetCurrentDialogueSet)
              (:%20%20
                (Variables|Default|SetUI 0)
                (Utilities|FlowControl|Sequence
                  (:then_0
                    (if (== _output_2 "Chadbro")
                      (bind _outactors (Actor|GetAllActorsOfClasswithTag "BP_NPC_C" "Punch Bowl"))
                      (Variables|BP_NPC_C|SetShouldSpeak (Utilities|Array|Get(acopy) _outactors) true)
                      (if (== (Variables|Default|GetCurrentDialogueSet) 2)
                        (Default|RemoveChecklistItem _checklist_4 "Speak to Chadbro")
                        (Default|AddChecklistItem _checklist_4 "Speak to Punch Bowl")
                        (elif (== (Variables|Default|GetCurrentDialogueSet) 3)
                          (bind _asbp_first_person_character_6 (Utilities|Casting|CastToBP_FirstPersonCharacter (Game|GetPlayerCharacter 0)))
                          (Math|Integer|IncrementInt (Variables|/Game/FirstPerson/Blueprints/BP_FirstPersonCharacter.BP_FirstPersonCharacter_C|GetOBJComplete _asbp_first_person_character_6)
                            (:%20%20
                              (Default|RemoveChecklistItem _checklist_4 "Speak to Chadbro")))))))
                  (:then_1
                    (if (== _output_2 "Punch Bowl")
                      (bind _outactors_2 (Actor|GetAllActorsOfClasswithTag "BP_NPC_C" "Chadbro"))
                      (Variables|BP_NPC_C|SetShouldSpeak (Utilities|Array|Get(acopy) _outactors_2) true)
                      (if (== (Variables|Default|GetCurrentDialogueSet) 2)
                        (Default|RemoveChecklistItem _checklist_2 "Speak to Punch Bowl")
                        (Default|AddChecklistItem _checklist_2 "Speak to Chadbro"))))
                  (:then_2
                    (if (== _output_2 "Stair Ghost")
                      (bind _outactors_3 (Actor|GetAllActorsOfClasswithTag "BP_NPC_C" "DJ"))
                      (Variables|BP_NPC_C|SetShouldSpeak (Utilities|Array|Get(acopy) _outactors_3) true)
                      (if (== (Variables|Default|GetCurrentDialogueSet) 2)
                        (Default|RemoveChecklistItem _checklist_5 "Speak to Stair Ghost")
                        (Default|AddChecklistItem _checklist_5 "Speak to DJ")
                        (elif (== (Variables|Default|GetCurrentDialogueSet) 3)
                          (bind _asbp_first_person_character_7 (Utilities|Casting|CastToBP_FirstPersonCharacter (Game|GetPlayerCharacter 0)))
                          (Math|Integer|IncrementInt (Variables|/Game/FirstPerson/Blueprints/BP_FirstPersonCharacter.BP_FirstPersonCharacter_C|GetOBJComplete _asbp_first_person_character_7)
                            (:%20%20
                              (Default|RemoveChecklistItem _checklist_5 "Speak to Stair Ghost")))))))
                  (:then_3
                    (if (== _output_2 "DJ")
                      (bind _outactors_4 (Actor|GetAllActorsOfClasswithTag "BP_NPC_C" "Stair Ghost"))
                      (Variables|BP_NPC_C|SetShouldSpeak (Utilities|Array|Get(acopy) _outactors_4) true)
                      (bind _outactors_5 (Actor|GetAllActorsOfClass "/Script/Engine.AmbientSound"))
                      (Audio|Components|Audio|SetSound (Variables|/Script/Engine.AmbientSound|GetAudioComponent (Utilities|Array|Get(acopy) _outactors_5)) "/Game/Audio/intenser_sounding.intenser_sounding")
                      (if (== (Variables|Default|GetCurrentDialogueSet) 2)
                        (Default|RemoveChecklistItem _checklist_3 "Speak to DJ")
                        (Default|AddChecklistItem _checklist_3 "Speak to Stair Ghost"))))
                  (:then_4
                    (if (== _output_2 "The Twins")
                      (if (== (Variables|Default|GetCurrentDialogueSet) 2)
                        (Default|RemoveChecklistItem _checklist "Speak to The Twins")
                        (Default|AddChecklistItem _checklist "Find a Slice")
                        (elif (== (Variables|Default|GetCurrentDialogueSet) 3)
                          (bind _asbp_first_person_character_8 (Utilities|Casting|CastToBP_FirstPersonCharacter (Game|GetPlayerCharacter 0)))
                          (Math|Integer|IncrementInt (Variables|/Game/FirstPerson/Blueprints/BP_FirstPersonCharacter.BP_FirstPersonCharacter_C|GetOBJComplete _asbp_first_person_character_8)
                            (:%20%20
                              (Default|RemoveChecklistItem _checklist "Speak to The Twins"))))))))))))))))

(fn ConstructionScript)