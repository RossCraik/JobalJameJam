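; Ghost face actor that animates eyes, mouth and brows on a test mesh by switching sprite indices in dynamic material instances.
; Tick timers drive randomized blinking, with low eye indices as blink frames, and random mouth frames while talking.
; EyesChange stores open-eye indices and defers them during a blink; each Change function lazily creates its material instance.
; ToggleTalking switches speech; debug keys toggle talking and randomize brows.
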(event EventBeginPlay
  (CallFunction|EyesChange (Math|Random|RandomIntegerinRange (+ (Variables|Default|Getblink_index_range) 1) 3))
  (CallFunction|MouthChange)
  (CallFunction|BrowsChange (Math|Random|RandomIntegerinRange 0 6)))

(event Collision|EventActorBeginOverlap
  (params (OtherActor :type Actor%20Object%20Reference)))

(event EventTick
  (params (DeltaSeconds :type Float%20%28single-precision%29))
  (Utilities|FlowControl|Sequence
    (:then_0
      (bind _output_get (Variables|Default|Setcurrent_blink_timer (+ (Variables|Default|Getcurrent_blink_timer) (* DeltaSeconds (Variables|Default|Getblink_rate)))))
      (if (> _output_get 1.0)
        (bind _output_get_2 (Variables|Default|Setis_blinking (not (Variables|Default|Getis_blinking))))
        (if _output_get_2
          (Variables|Default|Setcurrent_blink_timer (Math|Random|RandomFloatinRange 0.8 0.9))
          (CallFunction|EyesChange (Math|Random|RandomIntegerinRange 0 (Variables|Default|Getblink_index_range)))
          (else
            (Variables|Default|Setcurrent_blink_timer (Math|Random|RandomFloatinRange -0.25 0.0))
            (if (Variables|Default|Getis_talking)
              (CallFunction|EyesChange (Variables|Default|Getcurrent_eye_index))
              (else
                (CallFunction|EyesChange (Math|Random|RandomIntegerinRange (+ (Variables|Default|Getblink_index_range) 1) 3))))))))
    (:then_1
      (if (Variables|Default|Getis_talking)
        (bind _output_get_3 (Variables|Default|Setcurrent_talk_timer (+ (Variables|Default|Getcurrent_talk_timer) (* DeltaSeconds (Variables|Default|Gettalk_rate)))))
        (if (> _output_get_3 1.0)
          (CallFunction|MouthChange (Math|Random|RandomIntegerinRange 0 3))
          (Variables|Default|Setcurrent_talk_timer (Math|Random|RandomFloatinRange 0.0 0.6)))))))

(event Input|KeyboardEvents|DebugKeyT
  (params (Key :type Key%20Structure) (ActionValue :type Input%20Action%20Value%20Structure))
  (:Pressed
    (bind _output_get (Variables|Default|Setis_talking (not (Variables|Default|Getis_talking))))
    (if (not _output_get)
      (CallFunction|MouthChange))))

(event Input|KeyboardEvents|DebugKeyE
  (params (Key :type Key%20Structure) (ActionValue :type Input%20Action%20Value%20Structure))
  (:Pressed
    (CallFunction|BrowsChange (Math|Random|RandomIntegerinRange 0 6))))

(fn ConstructionScript)

(fn EyesChange
  (params (EyeIndex :type Integer))
  (if (<= EyeIndex (Variables|Default|Getblink_index_range))
    (if (Utilities|IsValid (Variables|Default|GetEyesMaterialInstance)) :!label _label
      _
      (else
        (bind _returnvalue (Rendering|Material|CreateDynamicMaterialInstance (Variables|Default|GetMesh_TestGhostFace) 0 "/Game/GhostFace/Mat_GhostEyes.Mat_GhostEyes" "None" :!class /Script/Engine.PrimitiveComponent))
        (bind _output_get (Variables|Default|SetEyesMaterialInstance _returnvalue))
        (Rendering|Material|SetTextureParameterValue _output_get "EyesTexture" (Variables|Default|GetEyesTexture))))
    (Rendering|Material|SetScalarParameterValue (Variables|Default|GetEyesMaterialInstance) "Index" (Math|Conversions|ToFloat(Integer) EyeIndex) :!class /Script/Engine.MaterialInstanceDynamic)
    (Rendering|Material|SetScalarParameterValue (Variables|Default|GetEyesMaterialInstance) "EyeCount" (Math|Conversions|ToFloat(Integer) (Variables|Default|GetEyeSpriteCount)) :!class /Script/Engine.MaterialInstanceDynamic)
    (else
      (Variables|Default|Setcurrent_eye_index EyeIndex)
      (if (not (Variables|Default|Getis_blinking))
        (Variables|Default|Setcurrent_blink_timer (+ (Variables|Default|Getcurrent_blink_timer) (Math|Random|RandomFloatinRange 0.0 0.2)))
        (goto _label)))))

(fn MouthChange
  (params (MouthIndex :type Integer))
  (Variables|Default|Setcurrent_mouth_index MouthIndex)
  (if (Utilities|IsValid (Variables|Default|GetMouthMaterialInstance))
    _
    (else
      (bind _returnvalue (Rendering|Material|CreateDynamicMaterialInstance (Variables|Default|GetMesh_TestGhostFace) 1 "/Game/GhostFace/Mat_GhostMouth.Mat_GhostMouth" "None" :!class /Script/Engine.PrimitiveComponent))
      (bind _output_get (Variables|Default|SetMouthMaterialInstance _returnvalue))
      (Rendering|Material|SetTextureParameterValue _output_get "MouthTexture" (Variables|Default|GetMouthTexture))))
  (Rendering|Material|SetScalarParameterValue (Variables|Default|GetMouthMaterialInstance) "Index" (Math|Conversions|ToFloat(Integer) MouthIndex) :!class /Script/Engine.MaterialInstanceDynamic)
  (Rendering|Material|SetScalarParameterValue (Variables|Default|GetMouthMaterialInstance) "MouthCount" (Math|Conversions|ToFloat(Integer) (Variables|Default|GetMouthSpriteCount)) :!class /Script/Engine.MaterialInstanceDynamic))

(fn BrowsChange
  (params (EyeIndex :type Integer))
  (if (Utilities|IsValid (Variables|Default|GetBrowsMaterialInstance))
    _
    (else
      (bind _returnvalue (Rendering|Material|CreateDynamicMaterialInstance (Variables|Default|GetMesh_TestGhostFace) 2 "/Game/GhostFace/MatGhostBrows.MatGhostBrows" "None" :!class /Script/Engine.PrimitiveComponent))
      (Variables|Default|SetBrowsMaterialInstance _returnvalue)))
  (Rendering|Material|SetScalarParameterValue (Variables|Default|GetBrowsMaterialInstance) "Index" (Math|Conversions|ToFloat(Integer) EyeIndex) :!class /Script/Engine.MaterialInstanceDynamic))

(fn ToggleTalking
  (params (is_talk :type Boolean))
  (bind _output_get (Variables|Default|Setis_talking is_talk))
  (if (not _output_get)
    (CallFunction|MouthChange)))